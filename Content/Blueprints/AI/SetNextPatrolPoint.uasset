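; Behavior tree task that advances an AI's patrol target, stored in the NextPatrolPoint blackboard key.
; When the key holds a valid object, it casts it to PatrolPoint and stores that point's linked NextPoint, following a chain through the level.
; Otherwise it seeds the key with the first PatrolPoint actor found in the world.
; Both branches finish successfully, but a failed cast never finishes the task.
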(event `self.ReceiveTickAI`
  (params (OwnerController :type "AIController Object Reference") (ControlledPawn :type "Pawn Object Reference") (DeltaSeconds :type "Float (single-precision)"))
  (bind _returnvalue (`AIBlueprintHelperLibrary.GetBlackboard` OwnerController))
  (bind _returnvalue_2 (`KismetStringLibrary.Conv_StringToName` "NextPatrolPoint"))
  (bind _returnvalue_3 (`BlackboardComponent.GetValueAsObject` _returnvalue _returnvalue_2))
  (if (`KismetSystemLibrary.IsValid` _returnvalue_3)
    (bind _aspatrol_point (cast `/Game/Blueprints/AI/PatrolPoint` _returnvalue_3))
    (`BlackboardComponent.SetValueAsObject` _returnvalue _returnvalue_2 (`/Game/Blueprints/AI/PatrolPoint.NextPoint` _aspatrol_point))
    (`self.FinishExecute` true)
    (else
      (bind _outactors (`GameplayStatics.GetAllActorsOfClass` "/Game/Blueprints/AI/PatrolPoint.PatrolPoint_C"))
      (for _array_element _outactors
        (`BlackboardComponent.SetValueAsObject` _returnvalue _returnvalue_2 _array_element)
        (break))
      (`self.FinishExecute` true))))