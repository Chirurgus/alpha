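; BaseCover_BP is a cover object with two trigger boxes, each paired with an arrow that supplies the cover's facing.
; Box overlaps send IsCoverAvailableMessage, true with the arrow's world rotation on begin and false with zero rotation on end.
; Only CoverBox1's begin overlap targets the other actor; the remaining three events target the overlapped component.
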(event `self.CoverBox1.OnComponentBeginOverlap`
  (params (OverlappedComponent :type "PrimitiveComponent Object Reference") (OtherActor :type "Actor Object Reference") (OtherComp :type "PrimitiveComponent Object Reference") (OtherBodyIndex :type Integer) (bFromSweep :type Boolean) (SweepResult :type "HitResult Structure (by ref)"))
  (message `/Game/Blueprints/UI/CoverInterface_BP.IsCoverAvailable` OtherActor true (`SceneComponent.K2_GetComponentRotation` (`self.Arrow1`))))

(event `self.CoverBox1.OnComponentEndOverlap`
  (params (OverlappedComponent :type "PrimitiveComponent Object Reference") (OtherActor :type "Actor Object Reference") (OtherComp :type "PrimitiveComponent Object Reference") (OtherBodyIndex :type Integer))
  (message `/Game/Blueprints/UI/CoverInterface_BP.IsCoverAvailable` OverlappedComponent false (struct)))

(event `self.CoverBox2.OnComponentBeginOverlap`
  (params (OverlappedComponent :type "PrimitiveComponent Object Reference") (OtherActor :type "Actor Object Reference") (OtherComp :type "PrimitiveComponent Object Reference") (OtherBodyIndex :type Integer) (bFromSweep :type Boolean) (SweepResult :type "HitResult Structure (by ref)"))
  (message `/Game/Blueprints/UI/CoverInterface_BP.IsCoverAvailable` OverlappedComponent true (`SceneComponent.K2_GetComponentRotation` (`self.Arrow2`))))

(event `self.CoverBox2.OnComponentEndOverlap`
  (params (OverlappedComponent :type "PrimitiveComponent Object Reference") (OtherActor :type "Actor Object Reference") (OtherComp :type "PrimitiveComponent Object Reference") (OtherBodyIndex :type Integer))
  (message `/Game/Blueprints/UI/CoverInterface_BP.IsCoverAvailable` OverlappedComponent false (struct)))

(fn `UserConstructionScript`)